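; EnemyTimeManager holds a current time scale for enemies and applies temporary changes to it.
; SetEnemyTimeScale stores the new value, broadcasts it through the OnTimeScaleChanged dispatcher, and restarts a timer that lasts for the Duration variable.
; When the timer fires, RevertEnemyTimeScale restores the default scale and broadcasts again, so each new call replaces any pending revert.
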(event `SetEnemyTimeScale`
  (params (NewTimeScale :type "Float (double-precision)"))
  (bind _output_get (set `self.CurrentEnemyTimeScale` NewTimeScale))
  (`self.OnTimeScaleChanged` _output_get)
  (`KismetSystemLibrary.K2_ClearAndInvalidateTimerHandle` (`self.TimeScaleRevertHandle`))
  (bind _returnvalue (`KismetSystemLibrary.K2_SetTimerDelegate` (delegate `RevertEnemyTimeScale`) (`self.Duration`)))
  (set `self.TimeScaleRevertHandle` _returnvalue))

(event `RevertEnemyTimeScale`
  (bind _output_get (set `self.CurrentEnemyTimeScale` (`self.DefaultEnemyTimeScale`)))
  (`self.OnTimeScaleChanged` _output_get))

(fn `UserConstructionScript`)