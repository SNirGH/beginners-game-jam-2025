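; Base game mode that runs endless rounds of enemy waves, with each round's enemy count scaling exponentially from a base count and growth rate.
; A looping timer asks a single BP_EnemySpawner to spawn until the round's quota is reached.
; EventManager game state events track living enemies, ending the round when all are spawned and dead, then starting the next after a delay.
; Tick prints the current quota for debugging.
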(event `self.ReceiveBeginPlay`
  (`self.CalculateMaxEnemyCount`)
  (bind _asevent_manager (cast `/Game/Blueprints/Framework/EventManager` (`GameplayStatics.GetGameState`)))
  (bind _output_get (set `self.EventManager` _asevent_manager))
  (add `/Game/Blueprints/Framework/EventManager.OnEnemySpawned` _output_get (delegate `EnemySpawed`))
  (add `/Game/Blueprints/Framework/EventManager.OnEnemyDeath` (`self.EventManager`) (delegate `EnemyDeath`))
  (`self.StartSpawningRound`))

(event `EnemySpawed`
  (`/Engine/EditorBlueprintResources/StandardMacros.IncrementInt` (`self.CurrentEnemyCount`)))

(event `EnemyDeath`
  (bind _result (`/Engine/EditorBlueprintResources/StandardMacros.DecrementInt` (`self.CurrentEnemyCount`))
    (:`  `
      (if (and (<= _result 0) (>= (`self.EnemiesSpawnedThisRound`) (`self.MaxEnemyCount`)))
        (`self.EndRound`)))))

(event `StartSpawningRound`
  (bind _returnvalue (`KismetSystemLibrary.K2_SetTimerDelegate` (delegate `SpawnEnemies`) (`self.SpawnTimer`) true)))

(event `SpawnEnemies`
  (if (>= (`self.EnemiesSpawnedThisRound`) (`self.MaxEnemyCount`))
    (`KismetSystemLibrary.K2_ClearAndInvalidateTimerHandle` (stale `StartSpawningRound` _returnvalue))
    (else
      (bind _returnvalue (`GameplayStatics.GetActorOfClass` "/Game/Blueprints/Characters/Enemies/BP_EnemySpawner.BP_EnemySpawner_C"))
      (`/Game/Blueprints/Characters/Enemies/BP_EnemySpawner.SpawnEnemy` _returnvalue)
      (`/Engine/EditorBlueprintResources/StandardMacros.IncrementInt` (`self.EnemiesSpawnedThisRound`)))))

(event `StartRound`
  (`self.StartSpawningRound`))

(event `EndRound`
  (`/Engine/EditorBlueprintResources/StandardMacros.IncrementInt` (`self.Round`)
    (:`  `
      (set `self.EnemiesSpawnedThisRound` 0)
      (set `self.CurrentEnemyCount` 0)
      (`self.CalculateMaxEnemyCount`)
      (`KismetSystemLibrary.Delay` 10.0)
      (`self.StartRound`))))

(event `CalculateMaxEnemyCount`
  (set `self.MaxEnemyCount` (`KismetMathLibrary.FFloor` (* (`self.BaseEnemyCount`) (`KismetMathLibrary.MultiplyMultiply_FloatFloat` (`self.GrowthRate`) (`KismetMathLibrary.Conv_IntToDouble` (- (`self.Round`) 1)))))))

(event `self.ReceiveTick`
  (params (DeltaSeconds :type "Float (single-precision)"))
  (`KismetSystemLibrary.PrintString` (`KismetStringLibrary.Conv_IntToString` (`self.MaxEnemyCount`)) true true (struct :`G` 0.66 :`B` 1.0 :`A` 1.0) 2.0 "1"))

(fn `UserConstructionScript`)