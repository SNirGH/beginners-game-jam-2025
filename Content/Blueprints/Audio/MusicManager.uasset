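; Music manager Blueprint that plays the past and future timezone tracks and the transition stingers between them.
; Track events spawn 2D MetaSounds and cache the component as CurrentTrack so StopTrack can stop it.
; PlayTransition uses a FlipFlop to alternate direction, starting with future-to-past.
; Each transition's OnAudioFinished is rebound to fire the TransitionFinished dispatcher for external listeners.
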(event `PlayPastTrack`
  (bind _returnvalue (`GameplayStatics.SpawnSound2D` "/Game/Assets/Audio/MS_PastTrack.MS_PastTrack" 1.0 1.0 0.0 null false false))
  (set `self.CurrentTrack` _returnvalue))

(event `PlayPastToFutureTransition`
  (bind _returnvalue (`GameplayStatics.SpawnSound2D` "/Game/Assets/Audio/Timezone_Transition_to_Future_Mastered.Timezone_Transition_to_Future_Mastered" 1.0 1.0 0.0 null false false))
  (`self.BindTransitionFinished` _returnvalue))

(event `PlayFutureTrack`
  (bind _returnvalue (`GameplayStatics.SpawnSound2D` "/Game/Assets/Audio/MS_FutureTrack.MS_FutureTrack" 1.0 1.0 0.0 null false false))
  (set `self.CurrentTrack` _returnvalue))

(event `PlayFutureToPastTransition`
  (bind _returnvalue (`GameplayStatics.SpawnSound2D` "/Game/Assets/Audio/Timezone_Transition_to_past_Mastered_1.Timezone_Transition_to_past_Mastered_1" 1.0 1.0 0.0 null false false))
  (`self.BindTransitionFinished` _returnvalue))

(event `StopTrack`
  (bind _currenttrack (`self.CurrentTrack`)
    (:`then`
      (if (`AudioComponent.IsPlaying` _currenttrack)
        (`AudioComponent.Stop` (`self.CurrentTrack`))))
    (:`else`)))

(event `PlayTransition`
  (`/Engine/EditorBlueprintResources/StandardMacros.FlipFlop`
    (:`A`
      (`self.PlayFutureToPastTransition`))
    (:`B`
      (`self.PlayPastToFutureTransition`))))

(event `BindTransitionFinished`
  (params (`Audio Component` :type "AudioComponent Object Reference"))
  (clear `AudioComponent.OnAudioFinished` `Audio Component`)
  (add `AudioComponent.OnAudioFinished` `Audio Component` (delegate `BroadcastTransitionFinished`)))

(event `BroadcastTransitionFinished`
  (`self.TransitionFinished`))