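; Actor component that gives its owner two melee-style attacks, a forward attack and an area-of-effect attack, both dealing fixed damage through the target's HealthComponent.
; ForwardAttack sphere-traces ahead of the owner and damages the first hit, while AOEAttack runs a multi-sphere trace around the owner.
; The AOE uses a temporary HitActors list so each actor is damaged once per attack.
; Both traces ignore the owner and draw debug shapes.
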(event `ForwardAttack`
  (bind _returnvalue (`self.GetOwner`))
  (bind _returnvalue_2 (`Actor.K2_GetActorLocation` _returnvalue))
  (bind (_outhit _returnvalue_3) (`KismetSystemLibrary.SphereTraceSingleForObjects` _returnvalue_2 (+ _returnvalue_2 (* (`Actor.GetActorForwardVector` _returnvalue) 300.0)) 60.0 (`|MakeArray` "ObjectTypeQuery1" "ObjectTypeQuery3" "ObjectTypeQuery2" "ObjectTypeQuery6" :!type "EObjectTypeQuery Enum") false (`|MakeArray` (`self.GetOwner`)) "ForDuration"))
  (if _returnvalue_3
    (bind _returnvalue_4 (`Actor.GetComponentByClass` (`.HitActor` (`GameplayStatics.BreakHitResult` _outhit)) "/Game/Blueprints/Components/HealthComponent.HealthComponent_C"))
    (`/Engine/EditorBlueprintResources/StandardMacros.IsValid` _returnvalue_4
      (:`Is Valid`
        (`/Game/Blueprints/Components/HealthComponent.TakeDamage` _returnvalue_4 10.0)))))

(event `AOEAttack`
  (bind _returnvalue (`Actor.K2_GetActorLocation` (`self.GetOwner`)))
  (bind (_outhits _returnvalue_2) (`KismetSystemLibrary.SphereTraceMultiForObjects` _returnvalue _returnvalue 300.0 (`|MakeArray` "ObjectTypeQuery1" "ObjectTypeQuery3" "ObjectTypeQuery2" "ObjectTypeQuery6" :!type "EObjectTypeQuery Enum") false (`|MakeArray` (`self.GetOwner`)) "ForDuration"))
  (if _returnvalue_2
    (for _array_element _outhits
      (bind (_bblockinghit _binitialoverlap _time _distance _location _impactpoint _normal _impactnormal _physmat _hitactor) (`GameplayStatics.BreakHitResult` _array_element))
      (`/Engine/EditorBlueprintResources/StandardMacros.IsValid` _hitactor
        (:`Is Valid`
          (bind _returnvalue_3 (`Actor.GetComponentByClass` _hitactor "/Game/Blueprints/Components/HealthComponent.HealthComponent_C"))
          (`/Engine/EditorBlueprintResources/StandardMacros.IsValid` _returnvalue_3
            (:`Is Valid`
              (if (not (`BlueprintSetLibrary.Set_Contains` (`self.HitActors`) _hitactor))
                (`BlueprintSetLibrary.Set_Add` (`self.HitActors`) _hitactor)
                (`/Game/Blueprints/Components/HealthComponent.TakeDamage` _returnvalue_3 10.0)))))))
    (`BlueprintSetLibrary.Set_Clear` (`self.HitActors`))))