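; Actor component that tracks an actor's health and creates the matching health UI for players and other pawns.
; On BeginPlay it fills health, then adds a HUD to the viewport for player-controlled pawns or a screen-space healthbar widget component above other pawns.
; TakeDamage clamps health and fires the damage and health-changed dispatchers, plus the death dispatcher whenever health is at zero.
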(event `self.ReceiveBeginPlay`
  (bind _maxhealth (`self.MaxHealth`))
  (bind _output_get (set `self.Health` _maxhealth))
  (`self.OnHealthChanged` _output_get _maxhealth)
  (bind _aspawn (cast `Pawn` (`self.GetOwner`)))
  (if (`Pawn.IsPlayerControlled` _aspawn)
    (bind _returnvalue (`|CreateWidget` "/Game/Blueprints/UI/WBP_PlayerHUD.WBP_PlayerHUD_C" null (`self.GetOwner`)))
    (`UserWidget.AddToViewport` _returnvalue 0)
    (else
      (bind _returnvalue_2 (`|AddComponentByClass` (`self.GetOwner`) "/Script/UMG.WidgetComponent" false (`KismetMathLibrary.MakeTransform` (0.0 0.0 100.0))))
      (`WidgetComponent.SetDrawSize` _returnvalue_2 (150.0 15.0))
      (`WidgetComponent.SetWidgetSpace` _returnvalue_2 "Screen")
      (`PrimitiveComponent.SetCollisionEnabled` _returnvalue_2 "NoCollision")
      (bind _returnvalue_3 (`|CreateWidget` "/Game/Blueprints/UI/WBP_EnemyHealthbar.WBP_EnemyHealthbar_C" null (`self.GetOwner`)))
      (`WidgetComponent.SetWidget` _returnvalue_2 _returnvalue_3))))

(fn `GetHealth`
  (returns (Health :type "Float (double-precision)"))
  (return (`self.Health`)))

(fn `TakeDamage`
  (params (Damage :type "Float (double-precision)"))
  (bind _output_get (set `self.Health` (`KismetMathLibrary.FClamp` (- (`self.Health`) (`local.Damage`)) 0.0 (`self.MaxHealth`))))
  (`self.OnDamageTaken`)
  (`self.OnHealthChanged` (`self.Health`) (`self.MaxHealth`))
  (if (<= _output_get 0.0)
    (`self.OnDeath`)))