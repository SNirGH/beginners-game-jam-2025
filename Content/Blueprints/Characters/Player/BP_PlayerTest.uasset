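; Test player character that fires projectiles, performs an area attack and turns to face the mouse cursor.
; The Fire input and E key forward to AttackComponent, passing the projectile spawn transform for shots.
; Each tick, a cursor trace on the Visibility channel sets only the actor's yaw toward the hit point.
; When HealthComponent reports death, the actor destroys itself and removes all widgets.
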(event `EnhancedInput|/Game/Blueprints/Input/InputActions/IA_Fire`
  (params (ActionValue :type Boolean) (ElapsedSeconds :type "Float (double-precision)") (TriggeredSeconds :type "Float (double-precision)") (InputAction :type "InputAction Object Reference" :default "/Game/Blueprints/Input/InputActions/IA_Fire.IA_Fire"))
  ; Fire Projectile
  (:`Triggered`
    (`/Game/Blueprints/Components/AttackComponent.FireWeapon` (`self.AttackComponent`) (`SceneComponent.K2_GetComponentToWorld` (`self.ProjectileSpawn`)))))

(event `Key|E`
  (params (Key :type "Key Structure"))
  ; AOE Attack
  (:`Pressed`
    (`/Game/Blueprints/Components/AttackComponent.AOEAttack` (`self.AttackComponent`))))

(event `self.HealthComponent.OnDeath`
  ; Handle On Death
  (`self.K2_DestroyActor`)
  (`WidgetLayoutLibrary.RemoveAllWidgets`))

(event `self.ReceiveTick`
  (params (DeltaSeconds :type "Float (single-precision)"))
  ; Rotate the character towards the mouse cursor. Mouse cursor is tracked using a tarce.
  (`self.RotateTowardsMouseCursor`))

(fn `RotateTowardsMouseCursor`
  (bind (_returnvalue_roll _returnvalue_pitch) (`KismetMathLibrary.BreakRotator` (`self.K2_GetActorRotation`)))
  (bind (_returnvalue_roll_2 _returnvalue_pitch_2 _returnvalue_yaw) (`KismetMathLibrary.BreakRotator` (`KismetMathLibrary.FindLookAtRotation` (`self.K2_GetActorLocation`) (`.Location` (`GameplayStatics.BreakHitResult` (`PlayerController.GetHitResultUnderCursorByChannel` (`GameplayStatics.GetPlayerController` 0) "TraceTypeQuery1" true))))))
  (`self.K2_SetActorRotation` (`KismetMathLibrary.MakeRotator` _returnvalue_roll _returnvalue_pitch _returnvalue_yaw)))

(fn `UserConstructionScript`)