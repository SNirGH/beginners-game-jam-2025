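; Player character Blueprint that aims with the mouse cursor and attacks through an AttackComponent.
; Each tick, a visibility trace under the cursor sets TargetRotation, and only the ProjectileSpawn component turns to that yaw, keeping the actor's pitch and roll.
; IA_Fire fires the weapon from ProjectileSpawn's transform, while a hardcoded E key triggers an AOE attack.
; HealthComponent's OnDeath removes all widgets, switches to UI-only input and destroys the actor.
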(event `EnhancedInput|/Game/Blueprints/Input/InputActions/IA_Fire`
  (params (ActionValue :type Boolean) (ElapsedSeconds :type "Float (double-precision)") (TriggeredSeconds :type "Float (double-precision)") (InputAction :type "InputAction Object Reference" :default "/Game/Blueprints/Input/InputActions/IA_Fire.IA_Fire"))
  ; Fire Projectile
  (:`Triggered`
    (`/Game/Blueprints/Components/AttackComponent.FireWeapon` (`self.AttackComponent`) (`SceneComponent.K2_GetComponentToWorld` (`self.ProjectileSpawn`)))))

(event `Key|E`
  (params (Key :type "Key Structure"))
  ; AOE Attack
  (:`Pressed`
    (`/Game/Blueprints/Components/AttackComponent.AOEAttack` (`self.AttackComponent`))))

(event `self.HealthComponent.OnDeath`
  ; Handle On Death
  (`WidgetLayoutLibrary.RemoveAllWidgets`)
  (`WidgetBlueprintLibrary.SetInputMode_UIOnlyEx` (`GameplayStatics.GetPlayerController` 0) null "DoNotLock" true)
  (`self.K2_DestroyActor`))

(event `self.ReceiveTick`
  (params (DeltaSeconds :type "Float (single-precision)"))
  ; Rotate the character towards the mouse cursor. Mouse cursor is tracked using a tarce.
  (`self.RotateTowardsMouseCursor`))

(fn `RotateTowardsMouseCursor`
  (bind (_bblockinghit _binitialoverlap _time _distance _location) (`GameplayStatics.BreakHitResult` (`PlayerController.GetHitResultUnderCursorByChannel` (`GameplayStatics.GetPlayerController` 0) "TraceTypeQuery1" true)))
  (bind (_returnvalue_roll _returnvalue_pitch _returnvalue_yaw) (`KismetMathLibrary.BreakRotator` (`KismetMathLibrary.FindLookAtRotation` (`self.K2_GetActorLocation`) _location)))
  (if _bblockinghit
    (set `self.Target Rotation` _returnvalue_yaw)
    (`self.SnapPlayerToFacing`)))

(fn `SnapPlayerToFacing`
  (bind (_returnvalue_roll _returnvalue_pitch) (`KismetMathLibrary.BreakRotator` (`self.K2_GetActorRotation`)))
  (`SceneComponent.K2_SetWorldRotation` (`self.ProjectileSpawn`) (`KismetMathLibrary.MakeRotator` _returnvalue_roll _returnvalue_pitch (`self.Target Rotation`)) false false))

(fn `UserConstructionScript`)