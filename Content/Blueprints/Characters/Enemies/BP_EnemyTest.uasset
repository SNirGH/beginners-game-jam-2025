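; BP_EnemyTest is a test enemy character that reports its lifecycle to the EventManager found on the game state.
; It announces its spawn one tick after BeginPlay.
; When its HealthComponent fires OnDeath, it flags itself dead, destroys itself after a short delay and notifies the EventManager.
; Each tick it sets PlayerInAttackRange by checking whether the first player pawn is within a short fixed distance.
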(event `self.ReceiveBeginPlay`
  (bind _asevent_manager (cast `/Game/Blueprints/Framework/EventManager` (`GameplayStatics.GetGameState`)))
  (bind _output_get (set `self.EventManager` _asevent_manager))
  (`KismetSystemLibrary.DelayUntilNextTick`)
  (`/Game/Blueprints/Framework/EventManager.OnEnemySpawned` _output_get))

(event `self.HealthComponent.OnDeath`
  (set `self.Is Dead` true)
  (`KismetSystemLibrary.Delay` 0.1)
  (`self.K2_DestroyActor`)
  (`/Game/Blueprints/Framework/EventManager.OnEnemyDeath` (`self.EventManager`)))

(event `self.ReceiveTick`
  (params (DeltaSeconds :type "Float (single-precision)"))
  (bind _returnvalue (`GameplayStatics.GetPlayerPawn` 0))
  (`/Engine/EditorBlueprintResources/StandardMacros.IsValid` _returnvalue
    (:`Is Valid`
      (if (< (`KismetMathLibrary.VSize` (- (`self.K2_GetActorLocation` _returnvalue) (`self.K2_GetActorLocation`))) 100.0)
        (set `self.PlayerInAttackRange` true)
        (else
          (set `self.PlayerInAttackRange` false))))))

(fn `UserConstructionScript`)