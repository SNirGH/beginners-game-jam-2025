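; Enemy spawner that places a samurai enemy at a random navigable point around itself, away from the player.
; SpawnEnemy retries random nav-mesh points within a radius until one meets the minimum player distance, then passes it to ChooseEnemy at a fixed height.
; ChooseEnemy alternates by GM_Base round parity, spawning the enemy class from the Cyberpunk samurai data asset on odd rounds and Feudal on even.
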(event `SpawnEnemy`
  (bind _returnvalue (`GameplayStatics.GetPlayerPawn` 0))
  (`/Engine/EditorBlueprintResources/StandardMacros.IsValid` _returnvalue
    (:`Is Valid`
      (set `self.Player Location` (`self.K2_GetActorLocation` _returnvalue))
      (for _ (range (`self.MaxRetries`))
        (bind _randomlocation (`NavigationSystemV1.K2_GetRandomLocationInNavigableRadius` (`NavigationSystemV1.GetNavigationSystem`) (`self.K2_GetActorLocation`) (`self.SpawnRadius`) null "/Script/AIModule.NavFilter_AIControllerDefault"))
        (if (>= (`KismetMathLibrary.Vector_Distance` _randomlocation (`self.Player Location`)) (`self.MinDistanceFromPlayer`))
          (`self.ChooseEnemy` (`KismetMathLibrary.MakeVector` (.x _randomlocation) (.y _randomlocation) 100.0))
          (break))))))

(fn `ChooseEnemy`
  (params (SpawnLocation :type "Vector Structure"))
  (bind _asgm_base (cast `/Game/Blueprints/Framework/GM_Base` (`GameplayStatics.GetGameMode`)))
  (if (!= (mod (`/Game/Blueprints/Framework/GM_Base.Round` _asgm_base) 2) 0)
    (bind _output_get (set `self.EnemyData` "/Game/Blueprints/Characters/Enemies/Data/DA_CyberpunkSamurai.DA_CyberpunkSamurai"))
    (`|SpawnActorFromClass` (`/Game/Blueprints/Characters/Enemies/Data/EnemyData.EnemyClass` _output_get) (`KismetMathLibrary.MakeTransform` (`local.SpawnLocation`)) "Undefined" "MultiplyWithRoot" null null)
    (else
      (bind _output_get_2 (set `self.EnemyData` "/Game/Blueprints/Characters/Enemies/Data/DA_FeudalSamurai.DA_FeudalSamurai"))
      (`|SpawnActorFromClass` (`/Game/Blueprints/Characters/Enemies/Data/EnemyData.EnemyClass` _output_get_2) (`KismetMathLibrary.MakeTransform` (`local.SpawnLocation`)) "Undefined" "MultiplyWithRoot" null null))))

(fn `UserConstructionScript`)